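; BP_SlingshotRock is a rock actor in the enemy ability assets, apparently the projectile for a slingshot attack.
; On BeginPlay it picks random yaw, pitch and roll rates, which Tick scales by delta time to tumble the rock mesh in local space.
; A short delay after spawn switches the sphere collision to query-only.
; The graph itself holds no movement or hit logic.
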(event `self.ReceiveBeginPlay`
  (bind _returnvalue (`KismetMathLibrary.RandomFloatInRange` -360.0 3600.0))
  (set `self.YawRotationRate` _returnvalue)
  (set `self.PitchRotationRate` _returnvalue)
  (set `self.RollRotationRate` _returnvalue)
  (`KismetSystemLibrary.Delay` 0.1)
  (`PrimitiveComponent.SetCollisionEnabled` (`self.Sphere`) "QueryOnly"))

(event `self.ReceiveTick`
  (params (DeltaSeconds :type "Float (single-precision)"))
  (`SceneComponent.K2_AddLocalRotation` (`self.RockWesh`) (`KismetMathLibrary.MakeRotator` (* DeltaSeconds (`self.RollRotationRate`)) (* DeltaSeconds (`self.PitchRotationRate`)) (* DeltaSeconds (`self.YawRotationRate`))) false false))

(fn `UserConstructionScript`)